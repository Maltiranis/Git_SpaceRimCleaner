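; Enemy that turns to face the player, fires projectiles and awards score when killed.
; Tick yaws the Cube mesh toward the player's body.
; The Shoot event, not called in this graph, spawns a projectile and muzzle effect at Cube1, gated by a random startup delay and a random cooldown.
; AnyDamage reduces Life and, at zero, adds player score, spawns a death effect and destroys the actor.
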(event EventBeginPlay
  ;[1 1 1] Fire
  (Utilities|FlowControl|Delay (Math|Random|RandomFloatinRange 7.0 8.0))
  (Variables|Default|SetDelayBeginPlay true))

(event EventShoot
  (bind _cube1 (Variables|Default|GetCube1))
  (bind _returnvalue (Transformation|GetWorldTransform _cube1))
  ;[1 1 1] Fire
  (if (Variables|Default|GetDelayBeginPlay)
    (if (not (Variables|Default|GetIsShootingDelai))
      (Game|SpawnActorfromClass "/Game/Core/Characters/Projectile/BP_Projectile_Enemy04.BP_Projectile_Enemy04_C" (Math|Transform|MakeTransform (.location _returnvalue) (.rotation _returnvalue) "1,1,1") "Undefined" 0 0)
      (Effects|SpawnEmitteratLocation "/Game/Art/VFX/Particules/Enemy/Rocket/ps_ennemyRocket_muzzle.ps_ennemyRocket_muzzle" (.location _returnvalue) (.rotation _returnvalue))
      (Variables|Default|SetIsShootingDelai true)
      (Utilities|FlowControl|Delay (Math|Random|RandomFloatinRange 4.0 1e+01))
      (Variables|Default|SetIsShootingDelai false))))

(event EventTick
  (params (DeltaSeconds :type Float%20%28single-precision%29))
  (bind _cube (Variables|Default|GetCube))
  ;[1 1 1] Look At Player
  (bind _asbp_player_character (Utilities|Casting|CastToBP_PlayerCharacter (Game|GetPlayerCharacter 0)))
  (Transformation|SetWorldRotation _cube (Math|Rotator|MakeRotator 0.0 0.0 (.yaw (Math|Rotator|FindLookatRotation (Transformation|GetWorldLocation _cube) (Transformation|GetWorldLocation (Variables|/Game/Core/Characters/BP_PlayerCharacter.BP_PlayerCharacter_C|GetBody _asbp_player_character))))) false false))

(event Game|Damage|EventAnyDamage
  (params (Damage :type Float%20%28single-precision%29) (DamageType :type Damage%20Type%20Object%20Reference) (InstigatedBy :type Controller%20Object%20Reference) (DamageCauser :type Actor%20Object%20Reference))
  (bind _capsulecomponent (Variables|Default|GetCapsuleComponent))
  (bind _returnvalue (Transformation|GetWorldTransform _capsulecomponent))
  ;[1 1 1] Look At Player
  (Variables|Default|SetLife (- (Variables|Default|GetLife) Damage))
  (if (<= (- (Variables|Default|GetLife) Damage) 0.0)
    (bind _asbp_player_character (Utilities|Casting|CastToBP_PlayerCharacter (Game|GetPlayerCharacter 0)))
    (Variables|/Game/Core/Characters/BP_PlayerCharacter.BP_PlayerCharacter_C|SetScore _asbp_player_character (+ (Variables|/Game/Core/Characters/BP_PlayerCharacter.BP_PlayerCharacter_C|GetScore _asbp_player_character) 30))
    (Effects|SpawnEmitteratLocation "/Game/Art/VFX/Particules/Enemy/Death/ps_ennemy_Death.ps_ennemy_Death" (.location _returnvalue) (.rotation _returnvalue))
    (Actor|DestroyActor)))

(fn ConstructionScript
  (|CallParentFunction))