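; PatrolPoints is an AI Blueprint that holds a Waypoints array and eight numbered waypoint variables, apparently to define a patrol route.
; The event graph has a chain that adds each waypoint to the array in order, but nothing triggers it, so it never runs.
; BeginPlay and the construction script are empty, so this graph does not populate the array at runtime.
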(event EventBeginPlay)

(fn ConstructionScript)