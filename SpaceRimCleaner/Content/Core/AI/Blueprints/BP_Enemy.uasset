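; BP_Enemy is an enemy Blueprint with a life pool that is destroyed when damage depletes it.
; AnyDamage subtracts the incoming damage from Life and destroys the actor at zero or below.
; A Shoot event sets the capsule component's world location to its current position plus a zero offset, so it fires nothing and moves nothing.
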(event Custom|Shoot
  (Transformation|SetWorldLocation (Variables|Collision|GetCapsuleComponent) (+ (Transformation|GetWorldLocation (Variables|Collision|GetCapsuleComponent)) "0, 0, 0") false false))

(event Game|Damage|EventAnyDamage
  (params (Damage :type Float%20%28single-precision%29) (DamageType :type Damage%20Type%20Object%20Reference) (InstigatedBy :type Controller%20Object%20Reference) (DamageCauser :type Actor%20Object%20Reference))
  (Variables|Default|SetLife (- (Variables|Default|GetLife) Damage))
  (if (<= (- (Variables|Default|GetLife) Damage) 0.0)
    (Actor|DestroyActor)))

(fn ConstructionScript)