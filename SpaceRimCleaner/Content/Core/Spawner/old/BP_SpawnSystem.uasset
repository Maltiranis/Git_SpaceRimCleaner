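; Wave spawner actor that spawns enemy classes one at a time at its Sphere component's location.
; On BeginPlay it fills Wave01 with three example enemy types and starts a looping half-second timer after a pre-wave delay.
; Each tick of that timer spawns the next entry; once exhausted, it waits the wave duration, increments WaveIndex and replays Wave01.
; Cost-based wave assignment is only a stub that resets WaveCurrentCost.
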(event Custom|SpawnWaveAlgo
  ;[1 1 1] START
  (CallFunction|SpawnSystem))

(event Custom|SpawnSystem
  (bind _s_spawner (Variables|Default|GetS_Spawner))
  (bind _wave_01 (Utilities|Struct|BreakS_Spawner _s_spawner))
  ;[0 1 1] Spawn One
  (if (< (Variables|Default|GetSpawnIndent) (Utilities|Array|Length _wave_01))
    (Game|SpawnActorfromClass (Utilities|Array|Get(acopy) _wave_01 (Variables|Default|GetSpawnIndent)) (Math|Conversions|ToTransform(Vector) (Transformation|GetWorldLocation (Variables|Default|GetSphere))) "AlwaysSpawn" 0 0)
    (Variables|Default|SetSpawnIndent (+ (Variables|Default|GetSpawnIndent) 1))
    (else
      (Utilities|FlowControl|Delay (.WaveDuration (Utilities|Struct|BreakS_Spawner (Variables|Default|GetS_Spawner))))
      (Variables|Default|SetWaveIndex (+ (Variables|Default|GetWaveIndex) 1))
      (Variables|Default|SetSpawnIndent 0))))

(event Custom|WaveCompositor
  (bind _s_enemis (Variables|Default|GetS_Enemis))
  (bind _s_spawner (Variables|Default|GetS_Spawner))
  (bind (_enemi01 _enemi02 _enemi03) (Utilities|Struct|BreakS_Enemis _s_enemis))
  (bind _wave_01 (Utilities|Struct|BreakS_Spawner _s_spawner))
  ;[1 0 0] Compositor Example
  (Utilities|Array|AddUnique _wave_01 _enemi01)
  (Utilities|Array|AddUnique _wave_01 _enemi02)
  (Utilities|Array|AddUnique _wave_01 _enemi03))

(event Custom|AssignEnemiesToWaves
  ;[1 1 1] Spawning Extanded System
  (Variables|Default|SetWaveCurrentCost 0.0))

(event EventBeginPlay
  ;[1 1 1] START
  ;;[1 0 0] Example
  (CallFunction|WaveCompositor)
  (Utilities|Time|SetTimerbyEvent (delegate Custom|SpawnWaveAlgo) 0.5 true (.DelayBeforeWave (Utilities|Struct|BreakS_Spawner (Variables|Default|GetS_Spawner)))))

(event Collision|EventActorBeginOverlap
  (params (OtherActor :type Actor%20Object%20Reference)))

(event EventTick
  (params (DeltaSeconds :type Float%20%28single-precision%29)))

(fn ConstructionScript)