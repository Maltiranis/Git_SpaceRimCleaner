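; BP_SpawnSystem is a wave spawner that creates actors from a configured class list at its Sphere component's location.
; BeginPlay starts a looping half-second timer after the configured initial delay, spawning the next Wave01 entry on each tick.
; When the list is exhausted, it waits for the wave duration, increments WaveIndex and resets the spawn counter.
; WaveIndex never selects the list, so Wave01 repeats indefinitely.
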(event Custom|Spawning
  (bind _varstruct (Variables|Default|GetvarStruct))
  (bind _wave_01 (Utilities|Struct|BreakS_Spawner _varstruct))
  ;[1 1 1] Spawning System
  (if (< (Variables|Default|GetSpawnIndent) (Utilities|Array|Length _wave_01))
    (Game|SpawnActorfromClass (Utilities|Array|Get(acopy) _wave_01 (Variables|Default|GetSpawnIndent)) (Math|Conversions|ToTransform(Vector) (Transformation|GetWorldLocation (Variables|Default|GetSphere))) "AlwaysSpawn" 0 0)
    (Variables|Default|SetSpawnIndent (+ (Variables|Default|GetSpawnIndent) 1))
    (else
      (Utilities|FlowControl|Delay (.WaveDuration (Utilities|Struct|BreakS_Spawner (Variables|Default|GetvarStruct))))
      (Variables|Default|SetWaveIndex (+ (Variables|Default|GetWaveIndex) 1))
      (Variables|Default|SetSpawnIndent 0))))

(event EventBeginPlay
  (Utilities|Time|SetTimerbyEvent (delegate Custom|Spawning) 0.5 true (.DelayBeforeWave (Utilities|Struct|BreakS_Spawner (Variables|Default|GetvarStruct)))))

(event Collision|EventActorBeginOverlap
  (params (OtherActor :type Actor%20Object%20Reference)))

(event EventTick
  (params (DeltaSeconds :type Float%20%28single-precision%29)))

(fn ConstructionScript)