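; BP_SpawnerSatelite is a rotating obstacle spawner that periodically launches an object from a satellite-style emitter.
; Each tick it yaws its Scene component by one degree, independent of frame rate scaling, keeping pitch and roll at zero.
; After a short random delay at BeginPlay, a CanShoot gate spawns the first ClassObject entry at Scene1's transform, then re-arms after a longer random delay.
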(event EventBeginPlay
  (Utilities|FlowControl|Delay (Math|Random|RandomFloatinRange 2.0 4.0))
  (Variables|Default|SetCanShoot true))

(event EventTick
  (params (DeltaSeconds :type Float%20%28single-precision%29))
  (bind _scene (Variables|Default|GetScene))
  (bind _scene1 (Variables|Default|GetScene1))
  (bind _returnvalue (Transformation|GetWorldTransform _scene1))
  (Transformation|SetWorldRotation _scene (Math|Rotator|MakeRotator 0.0 0.0 (+ (.yaw (Transformation|GetWorldRotation _scene)) 1.0)) false false)
  (if (Variables|Default|GetCanShoot)
    (Variables|Default|SetCanShoot false)
    (Game|SpawnActorfromClass (Utilities|Array|Get(acopy) (Variables|Default|GetClassObject)) (Math|Transform|MakeTransform (.location _returnvalue) (.rotation _returnvalue) "1,1,1") "Undefined" 0 0)
    (Utilities|FlowControl|Delay (Math|Random|RandomFloatinRange 15.0 22.0))
    (Variables|Default|SetCanShoot true)))

(fn ConstructionScript)