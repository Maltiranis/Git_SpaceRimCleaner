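; Wave spawner that spawns budget-based waves of random enemies, starting a looping timer after a first-wave delay.
; Each Wave Calculus call advances the wave index and draws from three enemy types via GetEnemiParams until a pick exceeds the remaining budget.
; Queued enemies spawn at random spawn points with random offsets.
; The budget then grows by a multiplier that tapers as the wave index rises.
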(event EventBeginPlay
  (bind _s_spawner_wavealgo (Variables|Default|GetS_Spawner_WaveAlgo))
  (bind (_waveindex _firstwavetimer _standardwavetimer _startwavecost) (Utilities|Struct|BreakS_Spawner_WaveAlgo _s_spawner_wavealgo))
  ;[1 1 1] START
  ;;[1 1 1] Set MaxCount
  (Variables|Default|SetWaveCost _startwavecost)
  (Utilities|FlowControl|Delay _firstwavetimer)
  (Utilities|Time|SetTimerbyFunctionName 0 "Wave Calculus" _standardwavetimer true))

(event Collision|EventActorBeginOverlap
  (params (OtherActor :type Actor%20Object%20Reference)))

(event EventTick
  (params (DeltaSeconds :type Float%20%28single-precision%29)))

(fn ConstructionScript)

(fn WaveCalculus
  (bind _spawnpoints (Variables|Default|GetSpawnPoints))
  (bind _wavearray (Variables|Default|GetWaveArray))
  (bind _spawnpoints_2 (Variables|Default|GetSpawnPoints))
  (bind _randomoffset (Variables|Default|GetRandomOffset))
  (bind _returnvalue (Utilities|Array|Length _spawnpoints_2))
  (bind _returnvalue_2 (Utilities|Array|Length _wavearray))
  (bind _returnvalue_3 (Math|Random|RandomInteger _returnvalue))
  (bind _output (Utilities|Array|Get(acopy) _spawnpoints _returnvalue_3))
  (bind _returnvalue_4 (Transformation|GetActorTransform _output))
  ;[1 1 1] Wave++
  (Development|PrintString (Utilities|String|ToString(Integer) (Utilities|Struct|BreakS_Spawner_WaveAlgo (Variables|Default|GetS_Spawner_WaveAlgo))) true true "(R=0.751524,G=0.764046,B=1.000000,A=1.000000)")
  (Variables|Default|SetS_Spawner_WaveAlgo (Utilities|Struct|MakeS_Spawner_WaveAlgo (+ (Utilities|Struct|BreakS_Spawner_WaveAlgo (Variables|Default|GetS_Spawner_WaveAlgo)) 1) 1.0 2.0 50 0.2))
  ;[1 1 1] CountRest == MaxCount
  (Variables|Default|SetCountRest (Variables|Default|GetWaveCost))
  ;[1 1 1] Test Random Enemi
  (while (>= (- (Variables|Default|GetCountRest) (stale _cost)) 0)
    (bind (_classref _cost) (CallFunction|GetEnemiParams self))
    ;[1 1 1] Make the Wave
    (if (>= (- (Variables|Default|GetCountRest) _cost) 0)
      (Utilities|Array|Add (Variables|Default|GetWaveArray) _classref)
      (Variables|Default|SetCountRest (- (Variables|Default|GetCountRest) _cost))))
  (Variables|Default|SetCountRest 0)
  ;[1 1 1] Comment
  (bind _index (Utilities|FlowControl|ForLoopwithBreak 0 _returnvalue_2)
    (:LoopBody
      (if (<= _index _returnvalue_2)
        (Game|SpawnActorfromClass (Utilities|Array|Get(acopy) (Variables|Default|GetWaveArray) _index) (Math|Transform|MakeTransform (+ (Math|Vector|MakeVector (* (Math|Random|RandomFloatinRange -1.0 1.0) (.x _randomoffset)) (* (Math|Random|RandomFloatinRange -1.0 1.0) (.y _randomoffset)) (* (Math|Random|RandomFloatinRange -1.0 1.0) (.z _randomoffset))) (.location _returnvalue_4)) (.rotation _returnvalue_4) (.scale _returnvalue_4)) "AlwaysSpawn" 0 0)))
    (:Completed
      (Utilities|Array|Clear (Variables|Default|GetWaveArray))
      ;[1 1 1] WaveCost
      (Development|PrintString (Utilities|String|ToString(Integer) (Variables|Default|GetWaveCost)) true true "(R=0.726175,G=0.000000,B=1.000000,A=1.000000)")
      (Variables|Default|SetWaveCost (Math|Float|Round (* (Math|Conversions|ToFloat(Integer) (Variables|Default|GetWaveCost)) (+ (/ (Utilities|Struct|BreakS_Spawner_WaveAlgo (Variables|Default|GetS_Spawner_WaveAlgo)) (/ (Math|Conversions|ToFloat(Integer) (Utilities|Struct|BreakS_Spawner_WaveAlgo (Variables|Default|GetS_Spawner_WaveAlgo))) 2.0)) 1.0)))))))

(fn GetEnemiParams
  (bind _returnvalue (Math|Random|RandomIntegerinRange 0 2))
  (bind _s_spawner_enemialgo (Variables|Default|GetS_Spawner_EnemiAlgo))
  (bind (_enemi_s_1 _cost_s_1 _enemi_m_1 _cost_m_1 _enemi_l_1 _cost_l_1) (Utilities|Struct|BreakS_Spawner_EnemiAlgo _s_spawner_enemialgo))
  (return (Utilities|Select :Index _returnvalue :Option%200 _enemi_s_1 :Option%201 _enemi_m_1 :Option%202 _enemi_l_1) (Utilities|Select :Index _returnvalue :Option%200 _cost_s_1 :Option%201 _cost_m_1 :Option%202 _cost_l_1)))