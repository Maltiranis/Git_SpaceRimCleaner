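; BP_ObstacleBase is a destructible obstacle that hurts the player on contact and destroys itself 40 seconds after spawning.
; Overlapping the player's character applies damage, plays the death particle effect and destroys the obstacle shortly after.
; Incoming damage drains Life; at zero it plays the effect and always drops a weighted random power-up, mostly Life, otherwise Multiplicateur, FireRate, Speed or EMP.
; The mesh rotation logic is unconnected.
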(event OnComponentBeginOverlap(Capsule)
  (params (OverlappedComponent :type Primitive%20Component%20Object%20Reference) (OtherActor :type Actor%20Object%20Reference) (OtherComp :type Primitive%20Component%20Object%20Reference) (OtherBodyIndex :type Integer) (bFromSweep :type Boolean) (SweepResult :type Hit%20Result%20Structure%20%28by%20ref%29))
  (bind _capsule (Variables|Default|GetCapsule))
  (bind _returnvalue (Transformation|GetWorldTransform _capsule))
  (bind _asbp_player_character (Utilities|Casting|CastToBP_PlayerCharacter OtherActor))
  (Game|Damage|ApplyDamage _asbp_player_character 1.0 0 0)
  (Effects|SpawnEmitteratLocation "/Game/Art/VFX/Particules/Enemy/Death/ps_ennemy_Death.ps_ennemy_Death" (.location _returnvalue) (.rotation _returnvalue) "3.000000,3.000000,3.000000")
  (Utilities|FlowControl|Delay 0.1)
  (Actor|DestroyActor))

(event Game|Damage|EventAnyDamage
  (params (Damage :type Float%20%28single-precision%29) (DamageType :type Damage%20Type%20Object%20Reference) (InstigatedBy :type Controller%20Object%20Reference) (DamageCauser :type Actor%20Object%20Reference))
  (bind _capsule (Variables|Default|GetCapsule))
  (bind _returnvalue (Transformation|GetWorldTransform _capsule))
  (bind _returnvalue_2 (Transformation|GetWorldLocation _capsule))
  (bind _output_get (Variables|Default|SetLife (- (Variables|Default|GetLife) Damage)))
  (if (<= _output_get 0.0)
    (Effects|SpawnEmitteratLocation "/Game/Art/VFX/Particules/Enemy/Death/ps_ennemy_Death.ps_ennemy_Death" (.location _returnvalue) (.rotation _returnvalue) "3.000000,3.000000,3.000000")
    (switch int (Math|Random|RandomIntegerinRange 0 19)
      (:0
        ;[1 1 1] Life
        (Game|SpawnActorfromClass "/Game/Core/Obstacles/PowerUp/BP_PowerUpLife.BP_PowerUpLife_C" (Math|Transform|MakeTransform (Math|Vector|MakeVector (.x _returnvalue_2) (.y _returnvalue_2) 0.0) "0, 0, 0" "1,1,1") "Undefined" 0 0 :!label _label)
        (Actor|DestroyActor))
      (:1
        (goto _label))
      (:2
        (goto _label))
      (:3
        (goto _label))
      (:4
        (goto _label))
      (:5
        (goto _label))
      (:6
        (Game|SpawnActorfromClass "/Game/Core/Obstacles/PowerUp/BP_PowerUpMultiplicateur.BP_PowerUpMultiplicateur_C" (Math|Transform|MakeTransform (Math|Vector|MakeVector (.x _returnvalue_2) (.y _returnvalue_2) 0.0) "0, 0, 0" "1,1,1") "Undefined" 0 0 :!label _label_2)
        (Actor|DestroyActor))
      (:7
        (goto _label))
      (:8
        (goto _label))
      (:9
        (goto _label))
      (:10
        (goto _label))
      (:11
        (goto _label))
      (:12
        (goto _label))
      (:13
        (goto _label))
      (:14
        ;[1 1 1] FireRate
        (Game|SpawnActorfromClass "/Game/Core/Obstacles/PowerUp/BP_PowerUpFireRate.BP_PowerUpFireRate_C" (Math|Transform|MakeTransform (Math|Vector|MakeVector (.x _returnvalue_2) (.y _returnvalue_2) 0.0) "0, 0, 0" "1,1,1") "Undefined" 0 0)
        (Actor|DestroyActor))
      (:15
        ;[1 1 1] SPeed
        (Game|SpawnActorfromClass "/Game/Core/Obstacles/PowerUp/BP_PowerUpSPeed.BP_PowerUpSPeed_C" (Math|Transform|MakeTransform (Math|Vector|MakeVector (.x _returnvalue_2) (.y _returnvalue_2) 0.0) "0, 0, 0" "1,1,1") "Undefined" 0 0 :!label _label_3)
        (Actor|DestroyActor))
      (:16
        (goto _label_3))
      (:17
        ;[1 1 1] EMP
        (Game|SpawnActorfromClass "/Game/Core/Obstacles/PowerUp/BP_PowerUpEMP.BP_PowerUpEMP_C" (Math|Transform|MakeTransform (Math|Vector|MakeVector (.x _returnvalue_2) (.y _returnvalue_2) 0.0) "0, 0, 0" "1,1,1") "Undefined" 0 0 :!label _label_4)
        (Actor|DestroyActor))
      (:18
        (goto _label_4))
      (:19
        (goto _label_2)))))

(event EventBeginPlay
  (Utilities|FlowControl|Delay 4e+01)
  (Actor|DestroyActor))

(fn ConstructionScript)