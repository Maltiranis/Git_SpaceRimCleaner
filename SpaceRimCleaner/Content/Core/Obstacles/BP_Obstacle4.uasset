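; BP_Obstacle4 is a slowly spinning obstacle that moves at a randomized projectile speed and destroys itself after a timed lifespan.
; Capsule overlap damages the player or reacts to other tagged obstacles, bursting in a death particle effect and destroying itself.
; Incoming damage drains its Life, and on death it randomly either just disappears or also spawns a life power-up.
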(event OnComponentBeginOverlap(Capsule)
  (params (OverlappedComponent :type Primitive%20Component%20Object%20Reference) (OtherActor :type Actor%20Object%20Reference) (OtherComp :type Primitive%20Component%20Object%20Reference) (OtherBodyIndex :type Integer) (bFromSweep :type Boolean) (SweepResult :type Hit%20Result%20Structure%20%28by%20ref%29))
  (bind _capsule (Variables|Default|GetCapsule))
  (bind _capsule_2 (Variables|Default|GetCapsule))
  (bind _returnvalue (Transformation|GetWorldTransform _capsule))
  (bind _returnvalue_2 (Transformation|GetWorldTransform _capsule_2))
  (Utilities|FlowControl|Sequence
    (:then_0
      (bind _asbp_player_character (Utilities|Casting|CastToBP_PlayerCharacter OtherActor))
      (Game|Damage|ApplyDamage _asbp_player_character 1.0 0 0)
      (Effects|SpawnEmitteratLocation "/Game/Art/VFX/Particules/Enemy/Death/ps_ennemy_Death.ps_ennemy_Death" (.location _returnvalue_2) (.rotation _returnvalue_2) "3.000000,3.000000,3.000000")
      (Utilities|FlowControl|Delay 0.1)
      (Actor|DestroyActor))
    (:then_1
      (Utilities|IsValid OtherActor
        (:Is%20Valid
          (if (Actor|ActorHasTag OtherActor "Obstacle")
            (Effects|SpawnEmitteratLocation "/Game/Art/VFX/Particules/Enemy/Death/ps_ennemy_Death.ps_ennemy_Death" (.location _returnvalue) (.rotation _returnvalue) "3.000000,3.000000,3.000000")
            (Actor|DestroyActor)))))))

(event EventTick
  (params (DeltaSeconds :type Float%20%28single-precision%29))
  (bind _scene (Variables|Default|GetScene))
  (bind _returnvalue (Transformation|GetWorldRotation _scene))
  (Transformation|SetWorldRotation _scene (Math|Rotator|MakeRotator (+ (.roll _returnvalue) 0.2) (.pitch _returnvalue) (+ (.yaw _returnvalue) 0.1)) false false))

(event Game|Damage|EventAnyDamage
  (params (Damage :type Float%20%28single-precision%29) (DamageType :type Damage%20Type%20Object%20Reference) (InstigatedBy :type Controller%20Object%20Reference) (DamageCauser :type Actor%20Object%20Reference))
  (bind _capsule (Variables|Default|GetCapsule))
  (bind _returnvalue (Transformation|GetWorldTransform _capsule))
  (bind _returnvalue_2 (Transformation|GetWorldLocation _capsule))
  (bind _output_get (Variables|Default|SetLife (- (Variables|Default|GetLife) Damage)))
  (if (<= _output_get 0.0)
    (Effects|SpawnEmitteratLocation "/Game/Art/VFX/Particules/Enemy/Death/ps_ennemy_Death.ps_ennemy_Death" (.location _returnvalue) (.rotation _returnvalue) "3.000000,3.000000,3.000000")
    (switch int (Math|Random|RandomIntegerinRange 0 1)
      (:0
        ;[1 1 1] Desrtoy
        (Actor|DestroyActor))
      (:1
        ;[1 1 1] Life
        (Game|SpawnActorfromClass "/Game/Core/Obstacles/PowerUp/BP_PowerUpLife.BP_PowerUpLife_C" (Math|Transform|MakeTransform (Math|Vector|MakeVector (.x _returnvalue_2) (.y _returnvalue_2) 0.0) "0, 0, 0" "1,1,1") "Undefined" 0 0)
        (Actor|DestroyActor)))))

(event EventBeginPlay
  (bind _returnvalue (Math|Random|RandomFloatinRange 125.0 2.2e+02))
  (bind _projectilemovement (Variables|Default|GetProjectileMovement))
  (Variables|/Script/Engine.ProjectileMovementComponent|SetInitialSpeed _projectilemovement _returnvalue)
  (Variables|/Script/Engine.ProjectileMovementComponent|SetMaxSpeed _projectilemovement _returnvalue)
  (Utilities|FlowControl|Delay 7e+01)
  (Actor|DestroyActor))

(fn ConstructionScript
  (|CallParentFunction))