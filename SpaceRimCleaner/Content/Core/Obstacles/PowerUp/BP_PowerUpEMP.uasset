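; BP_PowerUpEMP is a timed pickup that adds one EMP munition to an overlapping BP_PlayerCharacter, then destroys itself.
; From BeginPlay, a looping timer pulses the capsule's scale up and down through a FlipFlop.
; After a configurable delay, a faster timer blinks the cube's visibility as an expiry warning, and the actor destroys itself when the blink duration ends.
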(event OnComponentBeginOverlap(Capsule)
  (params (OverlappedComponent :type Primitive%20Component%20Object%20Reference) (OtherActor :type Actor%20Object%20Reference) (OtherComp :type Primitive%20Component%20Object%20Reference) (OtherBodyIndex :type Integer) (bFromSweep :type Boolean) (SweepResult :type Hit%20Result%20Structure%20%28by%20ref%29))
  (bind _asbp_player_character (Utilities|Casting|CastToBP_PlayerCharacter OtherActor))
  (Variables|/Game/Core/Characters/BP_PlayerCharacter.BP_PlayerCharacter_C|SetEMPMunition _asbp_player_character (+ (Variables|/Game/Core/Characters/BP_PlayerCharacter.BP_PlayerCharacter_C|GetEMPMunition _asbp_player_character) 1))
  (Actor|DestroyActor))

(event Custom|Clignotement
  (bind _capsule (Variables|Default|GetCapsule))
  (bind _capsule_2 (Variables|Default|GetCapsule))
  (Utilities|FlowControl|FlipFlop
    (:A
      (Transformation|SetWorldScale3D _capsule (+ (Transformation|GetWorldScale _capsule) 1.0)))
    (:B
      (Transformation|SetWorldScale3D _capsule_2 (+ (Transformation|GetWorldScale _capsule_2) -1.0)))))

(event Custom|BeforeDie
  (Utilities|FlowControl|FlipFlop
    (:A
      (Rendering|SetVisibility (Variables|Default|GetCube) false false))
    (:B
      (Rendering|SetVisibility (Variables|Default|GetCube) true false))))

(event EventBeginPlay
  (Utilities|Time|SetTimerbyEvent (delegate Custom|Clignotement) 0.5 true)
  (Utilities|FlowControl|Delay (Variables|Default|GetDelayBeforeCignotement))
  (Utilities|Time|SetTimerbyEvent (delegate Custom|BeforeDie) 0.2 true)
  (Utilities|FlowControl|Delay (Variables|Default|GetDurationClignotement))
  (Actor|DestroyActor))

(fn ConstructionScript)