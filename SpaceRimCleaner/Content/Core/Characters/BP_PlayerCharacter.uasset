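; Player character with twin-stick controls, a rotatable shield, shop access and a simple life counter.
; Left-stick axes drive movement and smoothly turn the Body, while right-stick axes independently turn the shield Cube, both using RInterpTo with a dead zone.
; A FlipFlop swaps controller IDs between players 0 and 1 to switch characters.
; Keys open the WBP_Shop widget, and damage lowers Life, with only debug prints for health and defeat.
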(event Game|Damage|EventAnyDamage
  (params (Damage :type Float%20%28single-precision%29) (DamageType :type Damage%20Type%20Object%20Reference) (InstigatedBy :type Controller%20Object%20Reference) (DamageCauser :type Actor%20Object%20Reference))
  (bind _output_get (Variables|Default|SetLife (- (Variables|Default|GetLife) Damage)))
  (if (<= _output_get 0.0)
    (Development|PrintString "Loose")
    (else
      (Development|PrintString (Utilities|String|ToString(Float) _output_get)))))

(event Input|ActionEvents|InputActionSwitchCharacter
  (params (Key :type Key%20Structure :default "None"))
  (:Pressed
    (Utilities|FlowControl|FlipFlop
      (:A
        (Class|GameplayStatics|SetPlayerControllerID (Game|GetPlayerController 0) 1)
        (Class|GameplayStatics|SetPlayerControllerID (Game|GetPlayerController 1)))
      (:B
        (Class|GameplayStatics|SetPlayerControllerID (Game|GetPlayerController 0))
        (Class|GameplayStatics|SetPlayerControllerID (Game|GetPlayerController 1) 1)))))

(event Input|AxisEvents|InputAxisMoveForward
  (params (AxisValue :type Float%20%28single-precision%29))
  (bind _body (Variables|Default|GetBody))
  ;[1 1 1] Movement
  (Utilities|FlowControl|Sequence
    (:then_0
      (if (>= (Math|Vector|VectorLength (Math|Vector|MakeVector AxisValue (stale Input|AxisEvents|InputAxisMoveRight AxisValue) 0.0)) 0.25)
        (Transformation|SetWorldRotation _body (Math|Interpolation|RInterpTo (Transformation|GetWorldRotation _body) (Math|Conversions|RotationFromXVector (Math|Vector|MakeVector AxisValue (stale Input|AxisEvents|InputAxisMoveRight AxisValue) 0.0)) (Utilities|Time|GetWorldDeltaSeconds) 7.0) false false)))
    (:then_1
      (if (> (Math|Vector|VectorLength (Math|Vector|ClampVectorSize (Math|Vector|MakeVector AxisValue (stale Input|AxisEvents|InputAxisMoveRight AxisValue) 0.0) 0.0 1.0)) 0.0)
        (Pawn|Input|AddMovementInput (Math|Vector|ClampVectorSize (Math|Vector|MakeVector AxisValue (stale Input|AxisEvents|InputAxisMoveRight AxisValue) 0.0) 0.0 1.0) 1.0 false)))))

(event Input|AxisEvents|InputAxisMoveRight
  (params (AxisValue :type Float%20%28single-precision%29))
  (bind _body (Variables|Default|GetBody))
  ;[1 1 1] Movement
  (Utilities|FlowControl|Sequence
    (:then_0
      (if (>= (Math|Vector|VectorLength (Math|Vector|MakeVector (stale Input|AxisEvents|InputAxisMoveForward AxisValue) AxisValue 0.0)) 0.25)
        (Transformation|SetWorldRotation _body (Math|Interpolation|RInterpTo (Transformation|GetWorldRotation _body) (Math|Conversions|RotationFromXVector (Math|Vector|MakeVector (stale Input|AxisEvents|InputAxisMoveForward AxisValue) AxisValue 0.0)) (Utilities|Time|GetWorldDeltaSeconds) 7.0) false false)))
    (:then_1
      (if (> (Math|Vector|VectorLength (Math|Vector|ClampVectorSize (Math|Vector|MakeVector (stale Input|AxisEvents|InputAxisMoveForward AxisValue) AxisValue 0.0) 0.0 1.0)) 0.0)
        (Pawn|Input|AddMovementInput (Math|Vector|ClampVectorSize (Math|Vector|MakeVector (stale Input|AxisEvents|InputAxisMoveForward AxisValue) AxisValue 0.0) 0.0 1.0) 1.0 false)))))

(event Input|AxisEvents|InputAxisStickR_Forward
  (params (AxisValue :type Float%20%28single-precision%29))
  (bind _cube (Variables|Default|GetCube))
  ;[1 1 1] Shield
  (if (> (Math|Vector|VectorLength (Math|Vector|MakeVector AxisValue (* (stale Input|AxisEvents|InputAxisStickR_Right AxisValue) -1.0) 0.0)) 0.25)
    (Transformation|SetWorldRotation _cube (Math|Interpolation|RInterpTo (Transformation|GetWorldRotation _cube) (Math|Rotator|MakeRotfromX (Math|Vector|MakeVector AxisValue (* (stale Input|AxisEvents|InputAxisStickR_Right AxisValue) -1.0) 0.0)) (Utilities|Time|GetWorldDeltaSeconds) 7.0) false false)))

(event Input|AxisEvents|InputAxisStickR_Right
  (params (AxisValue :type Float%20%28single-precision%29))
  (bind _cube (Variables|Default|GetCube))
  ;[1 1 1] Shield
  (if (> (Math|Vector|VectorLength (Math|Vector|MakeVector (stale Input|AxisEvents|InputAxisStickR_Forward AxisValue) (* AxisValue -1.0) 0.0)) 0.25)
    (Transformation|SetWorldRotation _cube (Math|Interpolation|RInterpTo (Transformation|GetWorldRotation _cube) (Math|Rotator|MakeRotfromX (Math|Vector|MakeVector (stale Input|AxisEvents|InputAxisStickR_Forward AxisValue) (* AxisValue -1.0) 0.0)) (Utilities|Time|GetWorldDeltaSeconds) 7.0) false false)))

(event Input|KeyboardEvents|E
  (params (Key :type Key%20Structure :default "None"))
  (:Pressed
    (bind _returnvalue (UserInterface|CreateWidget "/Game/Core/Widget/WBP_Shop.WBP_Shop_C"))
    (UserInterface|Viewport|AddtoViewport _returnvalue 0)
    (Variables|/Script/Engine.PlayerController|SetbShowMouseCursor (Game|GetPlayerController 0) true)))

(event Input|KeyboardEvents|S
  (params (Key :type Key%20Structure :default "None"))
  (:Pressed
    (Utilities|IsValid (stale Input|KeyboardEvents|E _returnvalue)
      (:Is%20Valid
        (UserInterface|Viewport|AddtoViewport (stale Input|KeyboardEvents|E _returnvalue) 0)))))

(fn ConstructionScript)