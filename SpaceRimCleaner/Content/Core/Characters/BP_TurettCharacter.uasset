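; Player-controlled turret character that aims by smoothly rotating StartPivot1 from the StickR axis inputs and fires from StartRaycast1.
; The MoveForward axis acts as the trigger: positive runs a looping Shoot1 projectile timer, negative a ChargeShoot timer that spawns a big projectile at full charge.
; Centering the axis pauses both timers.
; Rocket and line-trace Laser functions exist, but their triggers, a charge reset and second-pivot aiming are unconnected.
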(event Input|ActionEvents|InputActionLeftTrigger
  (params (Key :type Key%20Structure :default "None")))

(event Input|AxisEvents|InputAxisMoveForward
  (params (AxisValue :type Float%20%28single-precision%29))
  (Utilities|FlowControl|Sequence
    (:then_0
      (if (not (Variables|Default|GetIsShooting?))
        (if (> AxisValue 0.0)
          (Utilities|Time|SetTimerbyFunctionName 0 "Shoot1" (Variables|Shoot1|GetS1_FireRate) true)
          (Variables|Default|SetIsShooting? true))))
    (:then_1
      (if (not (Variables|Default|GetIsShooting?))
        (if (< AxisValue 0.0)
          (Utilities|Time|SetTimerbyFunctionName 0 "ChargeShoot" (Variables|Shoot2|GetS2_SpeedCharge) true)
          (Variables|Default|SetIsShooting? true))))
    (:then_2
      (if (Math|Float|InRange(Float) AxisValue -0.5 0.5)
        (Class|KismetSystemLibrary|PauseTimer 0 "Shoot1")
        (Class|KismetSystemLibrary|PauseTimer 0 "ChargeShoot")
        (Variables|Default|SetIsShooting? false)))))

(event Input|AxisEvents|InputAxisMoveRight
  (params (AxisValue :type Float%20%28single-precision%29)))

(event Input|AxisEvents|InputAxisStickR_Forward
  (params (AxisValue :type Float%20%28single-precision%29))
  (bind _startpivot1 (Variables|Default|GetStartPivot1))
  ;[1 1 1] Turret Stick L
  (if (> (Math|Vector|VectorLength (Math|Vector|MakeVector (* AxisValue -1.0) (stale Input|AxisEvents|InputAxisStickR_Right AxisValue) 0.0)) 0.25)
    (Transformation|SetWorldRotation _startpivot1 (Math|Interpolation|RInterpTo (Transformation|GetWorldRotation _startpivot1) (Math|Rotator|MakeRotfromX (Math|Vector|MakeVector (* AxisValue -1.0) (stale Input|AxisEvents|InputAxisStickR_Right AxisValue) 0.0)) (Utilities|Time|GetWorldDeltaSeconds) 7.0) false false)))

(event Input|AxisEvents|InputAxisStickR_Right
  (params (AxisValue :type Float%20%28single-precision%29))
  (bind _startpivot1 (Variables|Default|GetStartPivot1))
  ;[1 1 1] Turret Stick L
  (if (> (Math|Vector|VectorLength (Math|Vector|MakeVector (* (stale Input|AxisEvents|InputAxisStickR_Forward AxisValue) -1.0) AxisValue 0.0)) 0.25)
    (Transformation|SetWorldRotation _startpivot1 (Math|Interpolation|RInterpTo (Transformation|GetWorldRotation _startpivot1) (Math|Rotator|MakeRotfromX (Math|Vector|MakeVector (* (stale Input|AxisEvents|InputAxisStickR_Forward AxisValue) -1.0) AxisValue 0.0)) (Utilities|Time|GetWorldDeltaSeconds) 7.0) false false)))

(fn ConstructionScript)

(fn ChargeShoot
  (bind _startraycast1 (Variables|Default|GetStartRaycast1))
  (bind _returnvalue (Transformation|GetWorldTransform _startraycast1))
  (Variables|Shoot2|SetCurrentChargeShoot (Math|Float|Clamp(Float) (+ (Variables|Shoot2|GetCurrentChargeShoot) 1e+01) 0.0 5e+01))
  (if (>= (Variables|Shoot2|GetCurrentChargeShoot) 5e+01)
    (Game|SpawnActorfromClass "/Game/Core/Characters/Projectile/BP_BigProjectile.BP_BigProjectile_C" (Math|Transform|MakeTransform (.location _returnvalue) (.rotation _returnvalue) "1,1,1") "Undefined" 0 0)
    (Variables|Shoot2|SetCurrentChargeShoot 0.0)))

(fn Shoot1
  (bind _startraycast1 (Variables|Default|GetStartRaycast1))
  (bind _returnvalue (Transformation|GetWorldTransform _startraycast1))
  (Game|SpawnActorfromClass "/Game/Core/Characters/Projectile/BP_Projectile.BP_Projectile_C" (Math|Transform|MakeTransform (.location _returnvalue) (.rotation _returnvalue) "1,1,1") "Undefined" 0 0))

(fn Laser
  (bind _startraycast1 (Variables|Default|GetStartRaycast1))
  (bind _returnvalue (Transformation|GetWorldLocation _startraycast1))
  (bind _outhit (Collision|LineTraceByChannel _returnvalue (+ _returnvalue (* (Math|Vector|GetForwardVector _startraycast1) 1e+03)) "TraceTypeQuery1" false 0 "None"))
  (Game|Damage|ApplyDamage (.HitActor (Collision|BreakHitResult _outhit)) 0.1 0 0))

(fn Rocket
  (bind _startraycast1 (Variables|Default|GetStartRaycast1))
  (bind _returnvalue (Transformation|GetWorldTransform _startraycast1))
  (Game|SpawnActorfromClass "/Game/Core/Characters/Projectile/BP_Rocket.BP_Rocket_C" (Math|Transform|MakeTransform (.location _returnvalue) (.rotation _returnvalue) "1,1,1") "Undefined" 0 0))