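; Enemy projectile actor that damages the player character on overlap and destroys itself after three seconds if still alive.
; Its Sphere overlap reacts only to BP_PlayerCharacter, ignoring other actors.
; Hits on the player's Shield component destroy the projectile harmlessly.
; Any other component hit applies damage and spawns a blaster hit emitter at the player's Body before destroying the projectile.
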(event OnComponentBeginOverlap(Sphere)
  (params (OverlappedComponent :type Primitive%20Component%20Object%20Reference) (OtherActor :type Actor%20Object%20Reference) (OtherComp :type Primitive%20Component%20Object%20Reference) (OtherBodyIndex :type Integer) (bFromSweep :type Boolean) (SweepResult :type Hit%20Result%20Structure%20%28by%20ref%29))
  (bind _asbp_player_character (Utilities|Casting|CastToBP_PlayerCharacter OtherActor))
  (if (== OtherComp (Variables|/Game/Core/Characters/BP_PlayerCharacter.BP_PlayerCharacter_C|GetShield _asbp_player_character))
    (Actor|DestroyActor)
    (else
      (Game|Damage|ApplyDamage _asbp_player_character 1.0 0 0)
      (Effects|SpawnEmitteratLocation "/Game/Art/VFX/Particules/Enemy/Blaster/ps_ennemyblaster_Hit.ps_ennemyblaster_Hit" (Transformation|GetWorldLocation (Variables|/Game/Core/Characters/BP_PlayerCharacter.BP_PlayerCharacter_C|GetBody _asbp_player_character)) "0, 0, 0" "3.000000,3.000000,3.000000")
      (Actor|DestroyActor))))

(event EventBeginPlay
  (Utilities|FlowControl|Delay 3.0)
  (Actor|DestroyActor))

(fn ConstructionScript)