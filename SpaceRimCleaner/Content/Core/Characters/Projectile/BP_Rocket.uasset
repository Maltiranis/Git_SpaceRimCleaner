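; BP_Rocket is a rocket projectile that deals area damage to enemies and obstacles when it explodes.
; Explode, which has no caller in this graph, enables overlap events on Sphere1, spawns a scaled-up hit emitter there, then destroys the actor after a short delay.
; Sphere1 overlaps damage BP_EnemyBase actors and deal a larger base damage to actors tagged Obstacle.
; A timed self-destruct chain is present but disconnected.
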(event OnComponentBeginOverlap(Sphere1)
  (params (OverlappedComponent :type Primitive%20Component%20Object%20Reference) (OtherActor :type Actor%20Object%20Reference) (OtherComp :type Primitive%20Component%20Object%20Reference) (OtherBodyIndex :type Integer) (bFromSweep :type Boolean) (SweepResult :type Hit%20Result%20Structure%20%28by%20ref%29))
  (Utilities|FlowControl|Sequence
    (:then_0
      (bind _asbp_enemy_base (Utilities|Casting|CastToBP_EnemyBase OtherActor))
      (Game|Damage|ApplyDamage _asbp_enemy_base 1.0 0 0))
    (:then_1
      (Utilities|IsValid OtherActor
        (:Is%20Valid
          (if (Actor|ActorHasTag OtherActor "Obstacle")
            (Game|Damage|ApplyDamage OtherActor 4.0 0 0)))))))

(event Custom|Explode
  (bind _sphere1 (Variables|Default|GetSphere1))
  (Variables|/Script/Engine.PrimitiveComponent|SetbGenerateOverlapEvents _sphere1 true)
  (Effects|SpawnEmitteratLocation "/Game/Art/VFX/Particules/Player/Rocket/ps_playerRocket_Hit.ps_playerRocket_Hit" (Transformation|GetWorldLocation _sphere1) "0, 0, 0" "5.000000,5.000000,5.000000")
  (Utilities|FlowControl|Delay 0.2)
  (Actor|DestroyActor))

(event EventBeginPlay)

(fn ConstructionScript)