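; BP_Ultimate4 is a short-lived ultimate attack actor that deals heavy damage to any actor overlapping its Sphere, except the player character.
; On spawn, a fast looping timer runs Scale by Time, and the actor destroys itself shortly afterward.
; Each tick of that timer widens the static mesh in X and Y and raises the Sphere in world Z, both clamped and swept.
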(event OnComponentBeginOverlap(Sphere)
  (params (OverlappedComponent :type Primitive%20Component%20Object%20Reference) (OtherActor :type Actor%20Object%20Reference) (OtherComp :type Primitive%20Component%20Object%20Reference) (OtherBodyIndex :type Integer) (bFromSweep :type Boolean) (SweepResult :type Hit%20Result%20Structure%20%28by%20ref%29))
  (if (not (== OtherActor (.AsBP%20Player%20Character (Utilities|Casting|CastToBP_PlayerCharacter (Game|GetPlayerCharacter 0)))))
    (Game|Damage|ApplyDamage OtherActor 1e+03 0 0)))

(event EventBeginPlay
  (Utilities|Time|SetTimerbyFunctionName 0 "Scale by Time" 0.009 true)
  (Utilities|FlowControl|Delay 1.5)
  (Actor|DestroyActor))

(fn ConstructionScript)

(fn ScalebyTime
  (bind _staticmesh (Variables|Default|GetStaticMesh))
  (bind _sphere (Variables|Default|GetSphere))
  (bind _returnvalue (Transformation|GetWorldTransform _staticmesh))
  (bind _returnvalue_2 (Transformation|GetWorldLocation _sphere))
  (Transformation|SetWorldTransform _staticmesh (Math|Transform|MakeTransform (.location _returnvalue) (.rotation _returnvalue) (Math|Vector|MakeVector (Math|Float|Clamp(Float) (+ (.x (.scale _returnvalue)) 15.0) 0.0 4e+02) (Math|Float|Clamp(Float) (+ (.y (.scale _returnvalue)) 15.0) 0.0 4e+02) (.z (.scale _returnvalue)))) true false)
  (Transformation|SetWorldLocation _sphere (Math|Vector|MakeVector (.x _returnvalue_2) (.y _returnvalue_2) (Math|Float|Clamp(Float) (+ (.z _returnvalue_2) 5e+01) -8e+03 0.0)) true false))