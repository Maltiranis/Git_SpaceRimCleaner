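; Charged projectile actor that damages what it overlaps and destroys itself three seconds after spawning.
; Seven sphere components each run an identical overlap handler that applies a small amount of damage to the other actor.
; When the sweep's hit actor is valid, each handler also spawns an enlarged blaster hit particle at that actor's location.
; Overlaps do not destroy the projectile, so several spheres can each damage the same target.
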(event OnComponentBeginOverlap(Sphere)
  (params (OverlappedComponent :type Primitive%20Component%20Object%20Reference) (OtherActor :type Actor%20Object%20Reference) (OtherComp :type Primitive%20Component%20Object%20Reference) (OtherBodyIndex :type Integer) (bFromSweep :type Boolean) (SweepResult :type Hit%20Result%20Structure%20%28by%20ref%29))
  (bind _hitactor (Collision|BreakHitResult SweepResult))
  (Game|Damage|ApplyDamage OtherActor 0.5 0 0)
  (Utilities|IsValid _hitactor
    (:Is%20Valid
      (Effects|SpawnEmitteratLocation "/Game/Art/VFX/Particules/Enemy/Blaster/ps_ennemyblaster_Hit.ps_ennemyblaster_Hit" (Transformation|GetActorLocation _hitactor) "0, 0, 0" "2.000000,2.000000,2.000000"))))

(event OnComponentBeginOverlap(Sphere8)
  (params (OverlappedComponent :type Primitive%20Component%20Object%20Reference) (OtherActor :type Actor%20Object%20Reference) (OtherComp :type Primitive%20Component%20Object%20Reference) (OtherBodyIndex :type Integer) (bFromSweep :type Boolean) (SweepResult :type Hit%20Result%20Structure%20%28by%20ref%29))
  (bind _hitactor (Collision|BreakHitResult SweepResult))
  (Game|Damage|ApplyDamage OtherActor 0.5 0 0)
  (Utilities|IsValid _hitactor
    (:Is%20Valid
      (Effects|SpawnEmitteratLocation "/Game/Art/VFX/Particules/Enemy/Blaster/ps_ennemyblaster_Hit.ps_ennemyblaster_Hit" (Transformation|GetActorLocation _hitactor) "0, 0, 0" "2.000000,2.000000,2.000000"))))

(event OnComponentBeginOverlap(Sphere4)
  (params (OverlappedComponent :type Primitive%20Component%20Object%20Reference) (OtherActor :type Actor%20Object%20Reference) (OtherComp :type Primitive%20Component%20Object%20Reference) (OtherBodyIndex :type Integer) (bFromSweep :type Boolean) (SweepResult :type Hit%20Result%20Structure%20%28by%20ref%29))
  (bind _hitactor (Collision|BreakHitResult SweepResult))
  (Game|Damage|ApplyDamage OtherActor 0.5 0 0)
  (Utilities|IsValid _hitactor
    (:Is%20Valid
      (Effects|SpawnEmitteratLocation "/Game/Art/VFX/Particules/Enemy/Blaster/ps_ennemyblaster_Hit.ps_ennemyblaster_Hit" (Transformation|GetActorLocation _hitactor) "0, 0, 0" "2.000000,2.000000,2.000000"))))

(event OnComponentBeginOverlap(Sphere10)
  (params (OverlappedComponent :type Primitive%20Component%20Object%20Reference) (OtherActor :type Actor%20Object%20Reference) (OtherComp :type Primitive%20Component%20Object%20Reference) (OtherBodyIndex :type Integer) (bFromSweep :type Boolean) (SweepResult :type Hit%20Result%20Structure%20%28by%20ref%29))
  (bind _hitactor (Collision|BreakHitResult SweepResult))
  (Game|Damage|ApplyDamage OtherActor 0.5 0 0)
  (Utilities|IsValid _hitactor
    (:Is%20Valid
      (Effects|SpawnEmitteratLocation "/Game/Art/VFX/Particules/Enemy/Blaster/ps_ennemyblaster_Hit.ps_ennemyblaster_Hit" (Transformation|GetActorLocation _hitactor) "0, 0, 0" "2.000000,2.000000,2.000000"))))

(event OnComponentBeginOverlap(Sphere12)
  (params (OverlappedComponent :type Primitive%20Component%20Object%20Reference) (OtherActor :type Actor%20Object%20Reference) (OtherComp :type Primitive%20Component%20Object%20Reference) (OtherBodyIndex :type Integer) (bFromSweep :type Boolean) (SweepResult :type Hit%20Result%20Structure%20%28by%20ref%29))
  (bind _hitactor (Collision|BreakHitResult SweepResult))
  (Game|Damage|ApplyDamage OtherActor 0.5 0 0)
  (Utilities|IsValid _hitactor
    (:Is%20Valid
      (Effects|SpawnEmitteratLocation "/Game/Art/VFX/Particules/Enemy/Blaster/ps_ennemyblaster_Hit.ps_ennemyblaster_Hit" (Transformation|GetActorLocation _hitactor) "0, 0, 0" "2.000000,2.000000,2.000000"))))

(event OnComponentBeginOverlap(Sphere3)
  (params (OverlappedComponent :type Primitive%20Component%20Object%20Reference) (OtherActor :type Actor%20Object%20Reference) (OtherComp :type Primitive%20Component%20Object%20Reference) (OtherBodyIndex :type Integer) (bFromSweep :type Boolean) (SweepResult :type Hit%20Result%20Structure%20%28by%20ref%29))
  (bind _hitactor (Collision|BreakHitResult SweepResult))
  (Game|Damage|ApplyDamage OtherActor 0.5 0 0)
  (Utilities|IsValid _hitactor
    (:Is%20Valid
      (Effects|SpawnEmitteratLocation "/Game/Art/VFX/Particules/Enemy/Blaster/ps_ennemyblaster_Hit.ps_ennemyblaster_Hit" (Transformation|GetActorLocation _hitactor) "0, 0, 0" "2.000000,2.000000,2.000000"))))

(event OnComponentBeginOverlap(Sphere7)
  (params (OverlappedComponent :type Primitive%20Component%20Object%20Reference) (OtherActor :type Actor%20Object%20Reference) (OtherComp :type Primitive%20Component%20Object%20Reference) (OtherBodyIndex :type Integer) (bFromSweep :type Boolean) (SweepResult :type Hit%20Result%20Structure%20%28by%20ref%29))
  (bind _hitactor (Collision|BreakHitResult SweepResult))
  (Game|Damage|ApplyDamage OtherActor 0.5 0 0)
  (Utilities|IsValid _hitactor
    (:Is%20Valid
      (Effects|SpawnEmitteratLocation "/Game/Art/VFX/Particules/Enemy/Blaster/ps_ennemyblaster_Hit.ps_ennemyblaster_Hit" (Transformation|GetActorLocation _hitactor) "0, 0, 0" "2.000000,2.000000,2.000000"))))

(event EventBeginPlay
  (Utilities|FlowControl|Delay 3.0)
  (Actor|DestroyActor))

(fn ConstructionScript)